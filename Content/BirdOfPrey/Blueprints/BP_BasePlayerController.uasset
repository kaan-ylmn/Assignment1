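; Base player controller that handles the pause menu, screen measurement and death-time firing state.
; Pause input creates the PauseMenu widget and pauses the game, unless already paused or on the game-over screen.
; CalcScreenDimensions deprojects opposite viewport corners to a fixed distance, passing world X/Y spans as height/width to the game mode's world camera.
; OnPlayerDeath records whether the pawn's weapon was firing in DiedWhileFiring, which Reset clears.
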(event `self.ReceiveBeginPlay`)

(event `/Game/BirdOfPrey/Blueprints/IResetInterface.Reset`
  ;[1 1 1] Handle resetting this actor
  (set `self.bDiedWhileFiring` false))

(event `InputAction|PauseMenu` :consume false :paused true
  (params (Key :type "Key Structure"))
  (:`Pressed`
    (bind _asbp_base_game_mode (cast `/Game/BirdOfPrey/Blueprints/BP_BaseGameMode` (`GameplayStatics.GetGameMode`)))
    (if (and (not (`/Game/BirdOfPrey/Blueprints/BP_BaseGameMode.IsGameOverScreen` _asbp_base_game_mode)) (not (`GameplayStatics.IsGamePaused`)))
      (bind _returnvalue (`|CreateWidget` "/Game/BirdOfPrey/UI/PauseMenu.PauseMenu_C" self))
      (`UserWidget.AddToViewport` _returnvalue 0)
      (`GameplayStatics.SetGamePaused` true))))

(fn `CalcScreenDimensions`
  (bind (_sizex _sizey) (`self.GetViewportSize`))
  (bind (_worldlocation _worlddirection) (`self.DeprojectScreenPositionToWorld` 0.0))
  (bind (_worldlocation_2 _worlddirection_2) (`self.DeprojectScreenPositionToWorld` (`KismetMathLibrary.Conv_IntToDouble` _sizex) (`KismetMathLibrary.Conv_IntToDouble` _sizey)))
  (bind (_returnvalue_x _returnvalue_y) (`KismetMathLibrary.BreakVector` (+ _worldlocation (* _worlddirection 1900.0))))
  (bind (_returnvalue_x_2 _returnvalue_y_2) (`KismetMathLibrary.BreakVector` (+ _worldlocation_2 (* _worlddirection_2 1900.0))))
  (bind _asbp_base_game_mode (cast `/Game/BirdOfPrey/Blueprints/BP_BaseGameMode` (`GameplayStatics.GetGameMode`)))
  (`/Game/BirdOfPrey/Blueprints/WorldCameraActor.SetScreenDimensions` (`/Game/BirdOfPrey/Blueprints/BP_BaseGameMode.GetWorldCameraActor` _asbp_base_game_mode) (`KismetMathLibrary.Abs` (- _returnvalue_x _returnvalue_x_2)) (`KismetMathLibrary.Abs` (- _returnvalue_y _returnvalue_y_2))))

(fn `OnPlayerDeath`
  (params (Killer :type "Controller Object Reference"))
  (bind _asbase_game_agent (cast `/Game/BirdOfPrey/Blueprints/BaseGameAgent` (`self.K2_GetPawn`)))
  (set `self.bDiedWhileFiring` (`/Game/BirdOfPrey/Blueprints/BP_BaseWeapon.IsFiring` (`/Game/BirdOfPrey/Blueprints/BaseGameAgent.Weapon` _asbase_game_agent))))

(fn `UserConstructionScript`)