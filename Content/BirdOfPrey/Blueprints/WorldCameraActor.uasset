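; World camera actor that scrolls the view through the level and follows the player ship sideways.
; Each tick moves the actor by the game mode's world scroll velocity and eases the camera offset component toward the ship's clamped Y position.
; Despite its name, the averaging function uses only the first ship, keeping the last known value when none exist.
; Also provides reset to start, distance travelled, view-target assignment and screen dimensions.
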(event `self.ReceiveTick`
  (params (DeltaSeconds :type "Float (single-precision)"))
  (bind (_forward_movement_vector _horizontal_movement_vector) (`self.GetMovementVectors` DeltaSeconds))
  ;[1 1 1] Tick
  (`self.MoveActor` _forward_movement_vector) ; Move the view through the world
  (`self.MoveCameraOffset` _horizontal_movement_vector) ; Adjust the camera to compensate for player movement
)

(event `/Game/BirdOfPrey/Blueprints/IResetInterface.Reset`
  ;[1 1 1] Handle Reset
  (`self.K2_SetActorLocation` (`self.StartLocation`)))

(fn `CalculateAveragePlayerShipOffset`
  (params (PlayerShips :type "Array of /Game/BirdOfPrey/Blueprints/BP_PlayerShip Object Reference"))
  (returns (Offset :type "Float (double-precision)"))
  (bind (_returnvalue_x _returnvalue_y) (`KismetMathLibrary.BreakVector` (`self.K2_GetActorLocation` (`|GetArrayItem` PlayerShips))))
  (if (> (`KismetArrayLibrary.Array_Length` PlayerShips) 0)
    (set `self.LastKnowPlayerShipOffset` _returnvalue_y))
  (return (`self.LastKnowPlayerShipOffset`)))

(fn `CalculateForwardMovement`
  (params (DeltaTime :type "Float (double-precision)"))
  (returns (ForwardMovement :type "Vector Structure"))
  (return (* (`/Game/BirdOfPrey/Blueprints/BP_BaseGameMode.GetWorldScrollVelocity` (cast `/Game/BirdOfPrey/Blueprints/BP_BaseGameMode` (`GameplayStatics.GetGameMode`) :!pure true)) (`local.DeltaTime`))))

(fn `CalculateHorizontalMovement`
  (params (DeltaTime :type "Float (double-precision)"))
  (returns (`Return Value` :type "Vector Structure"))
  (bind _maxhorizontaloffset (`self.MaxHorizontalOffset`))
  (bind (_relativelocation_x _relativelocation_y) (`KismetMathLibrary.BreakVector` (`SceneComponent.RelativeLocation` (`self.CameraOffsetComponent`))))
  (bind _outactors (`GameplayStatics.GetAllActorsOfClass` "/Game/BirdOfPrey/Blueprints/BP_PlayerShip.BP_PlayerShip_C"))
  (bind _offset (`self.CalculateAveragePlayerShipOffset` _outactors))
  (return (`KismetMathLibrary.MakeVector` 0.0 (- (`KismetMathLibrary.FInterpTo` _relativelocation_y (`KismetMathLibrary.FClamp` _offset (* _maxhorizontaloffset -1.0) _maxhorizontaloffset) (`local.DeltaTime`) 15.0) _relativelocation_y))))

(fn `GetDistanceTravelled`
  (returns (ReturnValue :type "Float (double-precision)"))
  (bind _returnvalue_x (`KismetMathLibrary.BreakVector` (`self.K2_GetActorLocation`)))
  (bind _startlocation_x (`KismetMathLibrary.BreakVector` (`self.StartLocation`)))
  (return (`KismetMathLibrary.Abs` (- _returnvalue_x _startlocation_x))))

(fn `GetMovementVectors`
  (params (DeltaTime :type "Float (double-precision)"))
  (returns (`Forward Movement Vector` :type "Vector Structure") (`Horizontal Movement Vector` :type "Vector Structure"))
  (return (`self.CalculateForwardMovement` DeltaTime) (`self.CalculateHorizontalMovement` DeltaTime)))

(fn `GetScreenDimensions`
  (returns (Height :type "Float (double-precision)") (Width :type "Float (double-precision)"))
  (bind (_screendimensions_x _screendimensions_y) (`KismetMathLibrary.BreakVector2D` (`self.ScreenDimensions`)))
  (return _screendimensions_x _screendimensions_y))

(fn `MoveActor`
  (params (Amount :type "Vector Structure"))
  (`self.K2_SetActorLocation` (+ Amount (`self.K2_GetActorLocation`))))

(fn `MoveCameraOffset`
  (params (Amount :type "Vector Structure"))
  (`SceneComponent.K2_AddRelativeLocation` (`self.CameraOffsetComponent`) Amount false false))

(fn `SetPlayerViewCamera`
  (params (Target :type "PlayerController Object Reference"))
  (`PlayerController.SetViewTargetWithBlend` Target self 0.0 "VTBlend_Linear" 0.0 false))

(fn `SetScreenDimensions`
  (params (Height :type "Float (double-precision)") (Width :type "Float (double-precision)"))
  (set `self.ScreenDimensions` (`KismetMathLibrary.MakeVector2D` Height Width)))

(fn `UserConstructionScript`
  (set `self.StartLocation` (`self.K2_GetActorLocation`)))