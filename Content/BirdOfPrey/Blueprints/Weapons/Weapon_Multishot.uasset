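; Multishot weapon for Bird of Prey that lays out several projectiles side by side in an evenly spaced, parallel row.
; GetProjectileSpawnTransform maps each shot number to a position centered on the weapon, using NumShots and ShotOffset to space shots along the world Y axis.
; Every shot keeps the actor's rotation at unit scale, and the offset does not turn with the actor.
; The event graph holds no active logic.
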(fn `GetProjectileSpawnTransform`
  (params (`Shot Number` :type Integer))
  (returns (ReturnValue :type "Transform Structure"))
  (bind (_returnvalue_x _returnvalue_y _returnvalue_z) (`KismetMathLibrary.BreakVector` (`self.K2_GetActorLocation`)))
  (return (`KismetMathLibrary.MakeTransform` (`KismetMathLibrary.MakeVector` _returnvalue_x (+ (- _returnvalue_y (/ (* (- (`self.NumShots`) 1) (`self.ShotOffset`)) 2.0)) (* (- (`local.Shot Number`) 1) (`self.ShotOffset`))) _returnvalue_z) (`self.K2_GetActorRotation`))))

(fn `UserConstructionScript`
  (`parent.UserConstructionScript`))