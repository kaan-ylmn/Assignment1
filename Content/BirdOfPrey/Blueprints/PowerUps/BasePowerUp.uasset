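; Base power-up actor that the player ship collects by flying into it.
; On overlap with BP_PlayerShip it calls Apply, an empty hook for subclasses, plays a fixed pickup sound and destroys itself.
; PlayEffects spawns a particle and sound from variables, but nothing in this Blueprint calls it.
; The Reset event also destroys the actor, clearing uncollected pickups.
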(event `self.ReceiveActorBeginOverlap`
  (params (OtherActor :type "Actor Object Reference"))
  ;[1 1 1] Pick up on overlap
  (bind _asplayer_ship (cast `/Game/BirdOfPrey/Blueprints/BP_PlayerShip` OtherActor))
  (`self.Apply` _asplayer_ship)
  (`GameplayStatics.PlaySoundAtLocation` "/Game/BirdOfPrey/UI/PickupItem_Cue.PickupItem_Cue" (`self.K2_GetActorLocation`) (struct) 1.0 1.0 0.0 null null null null)
  (`self.K2_DestroyActor`))

(event `/Game/BirdOfPrey/Blueprints/IResetInterface.Reset`
  ;[1 1 1] Handle Reset
  (`self.K2_DestroyActor`))

(fn `Apply`
  (params (PlayerShip :type "/Game/BirdOfPrey/Blueprints/BP_PlayerShip Object Reference")))

(fn `PlayEffects`
  (`GameplayStatics.SpawnEmitterAtLocation` (`self.PickUpParticleSystem`) (`self.K2_GetActorLocation`))
  (`GameplayStatics.PlaySoundAtLocation` (`self.PickUpSoundCue`) (`self.K2_GetActorLocation`) (struct) 1.0 1.0 0.0 null null null null))

(fn `UserConstructionScript`)