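; Base AI controller for enemy agents that aims and fires at player ships.
; On possess it caches the controlled agent and picks a random player controller as target.
; Each tick it aims at the target's living ship when aim updates are enabled, then starts firing after a refire delay and stops once the weapon finishes or is missing.
; Aim and fire commands are forwarded to the agent.
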(event `self.ReceivePossess`
  (params (PossessedPawn :type "Pawn Object Reference"))
  ;[0.4235 0.251 1] Once this AIcontroller(Brains) takes over a Pawn (Controllable actor), select a new 'enemy' target.
  (`parent.ReceivePossess` null)
  (set `self.ControlledAgent` (cast `/Game/BirdOfPrey/Blueprints/BaseGameAgent` (`self.K2_GetPawn`) :!pure true)) ; Cache controlled agent for ease of access
  (`self.SelectTarget`))

(event `self.ReceiveTick`
  (params (DeltaSeconds :type "Float (single-precision)"))
  ;[0.4235 0.251 1] Tick - Regularly check if this AIcontroller should update it's aim and, confirm/update the current firing state.
  (`|ExecutionSequence`
    (:`then_0`
      (if (`self.ShouldUpdateAim`)
        (`self.UpdateAim`)))
    (:`then_1`
      (`self.CheckFire`))))

(fn `AimAt`
  (params (`Aim Target` :type "Vector Structure"))
  (bind _controlledagent (`self.ControlledAgent`))
  ;[0.4235 0.251 1] Comment
  (`/Engine/EditorBlueprintResources/StandardMacros.IsValid` _controlledagent ; If i'm controlling an agent...
    (:`Is Valid`
      (`/Game/BirdOfPrey/Blueprints/BaseGameAgent.Aim At` _controlledagent (`local.Aim Target`)) ; ...I will send it the coordinates of a target.
    )))

(fn `CheckFire`
  ;[0.4235 0.251 1] The 'CheckFire' function determines if the actor is firing and then update the firing action based on the output of the 'ShouldStartFiring' and 'ShouldStopFiring' functions.
  (if (`self.bIsFiring`)
    ;;[0.4235 0.251 1] If the actor is already firing, should it continue to do so?
    (if (`self.ShouldStopFire`)
      (`self.StopFire`))
    (else
      ;;[0.4235 0.251 1] If it isn't already firing, should it start?
      (if (`self.ShouldStartFire`)
        (`self.StartFire`)))))

(fn `SelectTarget`
  ;[0.4235 0.251 1] Randomly select a player to target from the list of players [Support for multiple players if extended however currently only ever has 1]
  (bind _outactors (`GameplayStatics.GetAllActorsOfClass` "/Game/BirdOfPrey/Blueprints/BP_BasePlayerController.BP_BasePlayerController_C"))
  (set `self.Target` (`|GetArrayItem` _outactors (`KismetMathLibrary.RandomInteger` (`KismetArrayLibrary.Array_Length` _outactors)))))

(fn `ShouldStartFire`
  (returns (ReturnValue :type Boolean))
  ;[0.4235 0.251 1] 'ShouldStartFire' function
  (return (> (- (`GameplayStatics.GetTimeSeconds`) (`self.LastFireTime`)) (`self.RefireDelay`))))

(fn `ShouldStopFire`
  (returns (ReturnValue :type Boolean))
  (bind _weapon (`/Game/BirdOfPrey/Blueprints/BaseGameAgent.Weapon` (`self.ControlledAgent`)))
  ;[0.4235 0.251 1] The 'ShouldStopFire' function is used to determine if the AIController should stop firing a weapon.
  (`/Engine/EditorBlueprintResources/StandardMacros.IsValid` _weapon ; Do I have a valid weapon?
    (:`Is Valid`
      (return (`/Game/BirdOfPrey/Blueprints/BP_BaseWeapon.HasFinishedFiring` _weapon)))
    (:`Is Not Valid`
      (return true) ; If not, then I shouldn't fire(Return TRUE)
    )))

(fn `ShouldUpdateAim`
  (returns (ReturnValue :type Boolean))
  (return (`self.bShouldUpdateAim`)))

(fn `StartFire`
  (bind _controlledagent (`self.ControlledAgent`))
  ;[0.4235 0.251 1] 'StartFire' function
  (`/Engine/EditorBlueprintResources/StandardMacros.IsValid` _controlledagent ; If i'm controlling an agent...
    (:`Is Valid`
      (`/Game/BirdOfPrey/Blueprints/BaseGameAgent.StartFire` _controlledagent) ; ...then I should tell it to start firing...
      (set `self.LastFireTime` (`GameplayStatics.GetTimeSeconds`)) ; ...and record the time that it started firing...
      (set `self.bIsFiring` true) ; ...as well as update my firing status.
    )))

(fn `StopFire`
  (bind _controlledagent (`self.ControlledAgent`))
  ;[0.4235 0.251 1] 'StopFire' function
  (`/Engine/EditorBlueprintResources/StandardMacros.IsValid` _controlledagent ; If i'm controlling an agent...
    (:`Is Valid`
      (`/Game/BirdOfPrey/Blueprints/BaseGameAgent.StopFire` _controlledagent) ; ...then I should tell it to stop firing...
      (set `self.bIsFiring` false) ; ..and update my firing status.
    )))

(fn `UpdateAim`
  (bind _returnvalue (`self.K2_GetPawn` (`self.Target`)))
  ;[0.4235 0.251 1] Check to make sure the target is still alive, and if so, set the targets location as the new aim location.
  (bind _asbp_player_ship (cast `/Game/BirdOfPrey/Blueprints/BP_PlayerShip` _returnvalue)) ; Is my target a playership...
  (if (`/Game/BirdOfPrey/Blueprints/BaseGameAgent.IsAlive` _asbp_player_ship)
    (`self.AimAt` (`self.K2_GetActorLocation` _returnvalue)) ; If my target is a living playership then I will aim at its location.
  ))

(fn `UserConstructionScript`)