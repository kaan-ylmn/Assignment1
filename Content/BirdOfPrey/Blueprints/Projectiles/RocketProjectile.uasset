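; Rocket projectile that extends a parent projectile class so its smoke trail can fade out before the actor is destroyed.
; The CleanUpandDestroy override deactivates the SmokeTrail particles, hides the mesh and disables capsule collision.
; It defers the parent's cleanup and destroy logic until the particle system's OnSystemFinished callback fires.
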(event `self.ReceiveBeginPlay`
  (`parent.ReceiveBeginPlay`))

(event `self.CleanUpAndDestroy`
  (bind _smoketrail (`self.SmokeTrail`))
  ;[1 1 1] Disables visuals and collision and then destroys the projectile once the smoke has faded out completely.
  (`ActorComponent.Deactivate` _smoketrail)
  (add `ParticleSystemComponent.OnSystemFinished` _smoketrail (delegate `OnSmokeFinished`))
  (`SceneComponent.SetVisibility` (`self.Mesh`) false false)
  (`PrimitiveComponent.SetCollisionEnabled` (`self.Capsule`) "NoCollision"))

(event `OnSmokeFinished`
  (params (PSystem :type "ParticleSystemComponent Object Reference"))
  ;[1 1 1] Disables visuals and collision and then destroys the projectile once the smoke has faded out completely.
  (`parent.CleanUpAndDestroy`))

(fn `UserConstructionScript`
  (`parent.UserConstructionScript`))